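; BP_Construction is a procedural building actor that assembles a flat facade of repeated wall modules from floor and segment counts.
; The Construction Script adds a static mesh component per cell in nested loops, spacing segments along X and floors along Z by the wall mesh's bounds.
; Each module receives frontal wall, side wall, window crystal and window frame materials.
; The event graph holds only disabled default events.
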(event EventBeginPlay)

(event Collision|EventActorBeginOverlap
  (params (OtherActor :type Actor%20Object%20Reference)))

(event EventTick
  (params (DeltaSeconds :type Float%20%28single-precision%29)))

(fn ConstructionScript
  (bind _wallmesh (Variables|Default|GetWallMesh))
  (bind _returnvalue (StaticMesh|GetBounds _wallmesh))
  (bind _boxextent (Math|BoxSphereBounds|BreakBoxSphereBounds _returnvalue))
  (bind (_x _y _z) (Math|Vector|BreakVector _boxextent))
  ;[1 1 1] For each building
  (for _index (range 0 (- (Variables|Default|GetNumberOfFloors) 1))
    ;[1 1 1] For each floor
    (for _index_2 (range 0 (- (Variables|Default|GetNumberOfSegments) 1))
      (bind _returnvalue_2 (AddComponent|AddStaticMeshComponent false (Math|Transform|MakeTransform (Math|Vector|MakeVector (* _index_2 (* _x 2.0)) 0.0 (* _index (* _z 2.0))))))
      (Components|StaticMesh|SetStaticMesh _returnvalue_2 (Variables|Default|GetWallMesh))
      (Rendering|Material|SetMaterial _returnvalue_2 0 (Variables|Default|GetFrontalWallMaterial))
      (Rendering|Material|SetMaterial _returnvalue_2 1 (Variables|Default|GetSideWallMaterial))
      (Rendering|Material|SetMaterial _returnvalue_2 2 (Variables|Default|GetWindowCrystalMaterial))
      (Rendering|Material|SetMaterial _returnvalue_2 3 (Variables|Default|GetWindowFrameMaterial)))))