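; BP_Pelican is a physics-simulated drone that follows an input-driven Cursor component.
; Movement axes offset the cursor and MoveRight yaws it, while Tick keeps it within CursorMaxDistance of the body.
; Tick also applies yaw torque scaled by the drone-to-cursor rotation difference and draws a debug arrow for cursor heading.
; BeginPlay enables physics and hands the skeletal mesh, cursor and an index to each of four propeller components.
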(event EventBeginPlay
  ;[1 1 1] We enable physics and collision and we initialize each propeller component
  (Physics|SetSimulatePhysics (Variables|Default|GetSK_Pelican) true)
  (Collision|SetCollisionEnabled (Variables|Default|GetSK_Pelican) "QueryAndPhysics")
  (bind _output_get (Variables|Default|SetPropellerComponents (Utilities|Array|MakeArray (Variables|Default|GetPropellerFL) (Variables|Default|GetPropellerFR) (Variables|Default|GetPropellerRR) (Variables|Default|GetPropellerRL))))
  (for (_array_element _array_index) _output_get
    (Default|InitComponent _array_element (Variables|Default|GetSK_Pelican) (Variables|Default|GetCursor) _array_index)))

(event EventTick
  (params (DeltaSeconds :type Float%20%28single-precision%29))
  (bind _cursor (Variables|Default|GetCursor))
  (bind _sk_pelican (Variables|Default|GetSK_Pelican))
  (bind _cursor_2 (Variables|Default|GetCursor))
  (bind _returnvalue (Transformation|GetWorldRotation _sk_pelican))
  (bind _returnvalue_2 (Transformation|GetWorldRotation _cursor))
  (bind _returnvalue_3 (Transformation|GetWorldLocation _cursor_2))
  (Class|PrimitiveComponent|AddTorque (Variables|Default|GetSK_Pelican) (Math|Vector|MakeVector 0.0 0.0 (Math|Float|Lerp 0.0 5e+02 (/ (.yaw (Class|KismetMathLibrary|NegateRotator (Math|Rotator|CombineRotators (Transformation|GetWorldRotation (Variables|Default|GetSK_Pelican)) (Class|KismetMathLibrary|NegateRotator (Transformation|GetWorldRotation (Variables|Default|GetCursor)))))) 1.8e+02))) "None" true)
  (Variables|Default|SetDroneRot _returnvalue)
  (Variables|Default|SetCursorRot _returnvalue_2)
  (Variables|Default|SetDrone+CursorRot (Class|KismetMathLibrary|NegateRotator (Math|Rotator|CombineRotators _returnvalue (Class|KismetMathLibrary|NegateRotator _returnvalue_2))))
  (Variables|Default|SetNewVar_1 (Math|Vector|GetForwardVector (Variables|Default|GetCursor)))
  (Rendering|Debug|DrawDebugArrow _returnvalue_3 (+ _returnvalue_3 (* (Math|Vector|GetForwardVector _cursor_2) 155.0)) 1e+01 "(R=1.000000,G=0.000000,B=0.855670,A=1.000000)" 0.0 3.0)
  (Transformation|SetWorldLocation (Variables|Default|GetCursor) (+ (Math|Vector|ClampVectorSize (- (Transformation|GetWorldLocation (Variables|Default|GetCursor)) (Transformation|GetWorldLocation (Variables|Default|GetSK_Pelican))) 0.0 (Variables|Default|GetCursorMaxDistance)) (Transformation|GetWorldLocation (Variables|Default|GetSK_Pelican))) false false))

(event Input|AxisEvents|InputAxisMoveForward
  (params (AxisValue :type Float%20%28single-precision%29))
  (Transformation|AddLocalOffset (Variables|Default|GetCursor) (Math|Vector|MakeVector (Math|Float|Lerp 0.0 5.0 AxisValue) (Math|Float|Lerp 0.0 5.0 (stale Input|AxisEvents|InputAxisMoveSide AxisValue)) (Math|Float|Lerp 0.0 5.0 (stale Input|AxisEvents|InputAxisMoveUp AxisValue))) false false))

(event Input|AxisEvents|InputAxisMoveSide
  (params (AxisValue :type Float%20%28single-precision%29))
  (Transformation|AddLocalOffset (Variables|Default|GetCursor) (Math|Vector|MakeVector (Math|Float|Lerp 0.0 5.0 (stale Input|AxisEvents|InputAxisMoveForward AxisValue)) (Math|Float|Lerp 0.0 5.0 AxisValue) (Math|Float|Lerp 0.0 5.0 (stale Input|AxisEvents|InputAxisMoveUp AxisValue))) false false))

(event Input|AxisEvents|InputAxisMoveUp
  (params (AxisValue :type Float%20%28single-precision%29))
  (Transformation|AddLocalOffset (Variables|Default|GetCursor) (Math|Vector|MakeVector (Math|Float|Lerp 0.0 5.0 (stale Input|AxisEvents|InputAxisMoveForward AxisValue)) (Math|Float|Lerp 0.0 5.0 (stale Input|AxisEvents|InputAxisMoveSide AxisValue)) (Math|Float|Lerp 0.0 5.0 AxisValue)) false false))

(event Input|AxisEvents|InputAxisMoveRight
  (params (AxisValue :type Float%20%28single-precision%29))
  (Transformation|AddLocalRotation (Variables|Default|GetCursor) (Math|Rotator|MakeRotator 0.0 0.0 (* AxisValue 2.0)) false false))

(fn ConstructionScript)