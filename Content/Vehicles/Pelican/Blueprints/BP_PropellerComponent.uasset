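; Propeller component for the Pelican drone that pushes its parent mesh toward a cursor component using physics.
; InitComponent stores drone, cursor and propeller index, whose parity sets spin direction.
; Each tick sums gravity hover, cursor-offset pitch, roll and lift, yaw matching and a local height correction into non-negative thrust.
; It applies this at the propeller's location along a skewed up vector, sets drone damping and draws a debug arrow.
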(event Custom|InitComponent
  (params (MeshComponent :type Skeletal%20Mesh%20Component%20Object%20Reference) (CursorComponent :type Scene%20Component%20Object%20Reference) (PropellerIndex :type Integer))
  ;[1 1 1] Get the parent component (drone), the cursor component and the propeller index
  (Variables|Default|SetParentComponent MeshComponent)
  (Variables|Default|SetCursorComponent CursorComponent)
  (bind _output_get (Variables|Default|SetPropellerIndex PropellerIndex))
  (Variables|Default|SetisCCW (Math|Conversions|ToBoolean(Integer) (Math|Integer|%(Integer) _output_get 2))))

(event EventTick
  (params (DeltaSeconds :type Float%20%28single-precision%29))
  (bind _returnvalue (Transformation|GetWorldTransform))
  (bind _returnvalue_2 (Math|Vector|GetForwardVector))
  (bind _returnvalue_3 (Transformation|GetWorldLocation))
  (bind _returnvalue_4 (Math|Vector|GetRightVector))
  (bind _returnvalue_5 (Math|Vector|GetUpVector))
  (bind _isccw (Variables|Default|GetisCCW))
  (bind _isccw_2 (Variables|Default|GetisCCW))
  (bind _cursormaxdistance (Variables|Default|GetCursorMaxDistance))
  (bind _propellerindex (Variables|Default|GetPropellerIndex))
  (bind _tiltmaxforce (Variables|Default|GetTiltMaxForce))
  (bind _parentcomponent (Variables|Default|GetParentComponent))
  (bind _upmaxforce (Variables|Default|GetUpMaxForce))
  (bind _cursorcomponent (Variables|Default|GetCursorComponent))
  (bind _parentcomponent_2 (Variables|Default|GetParentComponent))
  (bind _gravity (Variables|Default|GetGravity))
  (bind _numpropellers (Variables|Default|GetNumPropellers))
  (bind _cursorcomponent_2 (Variables|Default|GetCursorComponent))
  (bind _cursormaxdistance_2 (Variables|Default|GetCursorMaxDistance))
  (bind _cursormaxdistance_3 (Variables|Default|GetCursorMaxDistance))
  (bind _tiltmaxforce_2 (Variables|Default|GetTiltMaxForce))
  (bind _propellerindex_2 (Variables|Default|GetPropellerIndex))
  (bind _cursorcomponent_3 (Variables|Default|GetCursorComponent))
  (bind _parentcomponent_3 (Variables|Default|GetParentComponent))
  (bind _returnvalue_6 (Physics|GetMass _parentcomponent_2))
  (bind _returnvalue_7 (Transformation|GetWorldLocation _cursorcomponent_2))
  (bind _returnvalue_8 (* _returnvalue_2 -1e+01))
  (bind _returnvalue_9 (Transformation|GetWorldLocation _cursorcomponent_3))
  (bind _returnvalue_10 (Transformation|GetWorldTransform _parentcomponent_3))
  (bind _returnvalue_11 (Math|Float|SelectFloat 1.0 -1.0 _isccw))
  (bind _returnvalue_12 (Transformation|GetWorldRotation _parentcomponent))
  (bind _returnvalue_13 (Transformation|GetWorldRotation _cursorcomponent))
  (bind _returnvalue_14 (Math|Float|SelectFloat -1e+01 1e+01 _isccw_2))
  (bind _returnvalue_15 (Utilities|Select :Index _propellerindex :Option%200 1.0 :Option%201 -1.0 :Option%202 -1.0 :Option%203 1.0))
  (bind _returnvalue_16 (Utilities|Select :Index _propellerindex_2 :Option%200 -1.0 :Option%201 -1.0 :Option%202 1.0 :Option%203 1.0))
  (bind _returnvalue_17 (* _returnvalue_4 _returnvalue_14))
  (bind _returnvalue_18 (Math|Transform|InverseTransformLocation _returnvalue _returnvalue_7))
  (bind _returnvalue_19 (Math|Transform|InverseTransformLocation _returnvalue_10 _returnvalue_9))
  (bind _returnvalue_20 (Class|KismetMathLibrary|NegateRotator _returnvalue_13))
  (bind _returnvalue_21 (* _returnvalue_6 _gravity))
  (bind _returnvalue_22 (* _returnvalue_16 _tiltmaxforce))
  (bind _returnvalue_23 (* _returnvalue_15 _tiltmaxforce_2))
  (bind _returnvalue_24 (/ _returnvalue_21 _numpropellers))
  (bind _returnvalue_25 (/ (.x _returnvalue_19) _cursormaxdistance))
  (bind _returnvalue_26 (/ (.z _returnvalue_19) _cursormaxdistance_2))
  (bind _returnvalue_27 (/ (.y _returnvalue_19) _cursormaxdistance_3))
  (bind _returnvalue_28 (Math|Vector|VectorLength _returnvalue_18))
  (bind _z (Math|Vector|BreakVector _returnvalue_18))
  (bind _returnvalue_29 (Math|Rotator|CombineRotators _returnvalue_12 _returnvalue_20))
  (bind _returnvalue_30 (+ _returnvalue_17 _returnvalue_8 _returnvalue_5))
  (bind _returnvalue_31 (Math|Float|Lerp 0.0 _returnvalue_22 _returnvalue_25))
  (bind _returnvalue_32 (Math|Float|Lerp 0.0 _upmaxforce _returnvalue_26))
  (bind _returnvalue_33 (Math|Float|Lerp 0.0 _returnvalue_23 _returnvalue_27))
  (bind _returnvalue_34 (/ _z _returnvalue_28))
  (bind _returnvalue_35 (Class|KismetMathLibrary|NegateRotator _returnvalue_29))
  (bind _returnvalue_36 (< _returnvalue_34 -0.5))
  (bind _returnvalue_37 (> _returnvalue_34 0.5))
  (bind _returnvalue_38 (/ (.yaw _returnvalue_35) 1.8e+02))
  (bind _returnvalue_39 (+ _returnvalue_31 _returnvalue_33 _returnvalue_32))
  (bind _returnvalue_40 (Math|Float|Lerp 0.0 3e+03 _returnvalue_38))
  (bind _returnvalue_41 (or _returnvalue_36 _returnvalue_37))
  (bind _returnvalue_42 (Math|Float|SelectFloat _returnvalue_34 0.0 _returnvalue_41))
  (bind _returnvalue_43 (* _returnvalue_40 _returnvalue_11))
  (bind _returnvalue_44 (Math|Float|Lerp 0.0 1e+03 _returnvalue_42))
  (bind _returnvalue_45 (+ _returnvalue_24 _returnvalue_39 _returnvalue_43 _returnvalue_44))
  (bind _returnvalue_46 (Math|Float|Max(Float) _returnvalue_45 0.0))
  (bind _returnvalue_47 (* _returnvalue_30 _returnvalue_46))
  ;[1 1 1] Force direction debug arrow
  (Rendering|Debug|DrawDebugArrow _returnvalue_3 (+ _returnvalue_3 (* (Math|Vector|Normalize _returnvalue_47) 5e+01)) 8.0 "(R=0.023822,G=1.000000,B=0.000000,A=1.000000)" 0.0 2.0)
  ;[1 1 1] Apply the force to the propeller location and set the linear and angular damping of the drone
  (Class|PrimitiveComponent|AddForceatLocation (Variables|Default|GetParentComponent) _returnvalue_47 (Transformation|GetWorldLocation) "None")
  (Class|PrimitiveComponent|SetLinearDamping (Variables|Default|GetParentComponent) 3.0)
  (Class|PrimitiveComponent|SetAngularDamping (Variables|Default|GetParentComponent) 15.0)
  (Variables|Default|SetNewVar_0 (Math|Vector|MakeVector (.x _returnvalue_19) (.y _returnvalue_19) (.z _returnvalue_19)))
  (Variables|Default|SetNewVar_1 (Math|Vector|VectorLength _returnvalue_47)))