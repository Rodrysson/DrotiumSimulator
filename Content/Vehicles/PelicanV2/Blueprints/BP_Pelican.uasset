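; BP_Pelican is a physics-simulated drone that turns to follow an input-driven cursor.
; Move inputs offset and yaw the cursor, which Tick clamps within a maximum distance of the drone and marks with a debug arrow.
; Tick applies an upward force countering gravity and a yaw torque scaled by the rotation difference to the cursor.
; Positional force and roll/pitch torque calculations exist but are unconnected, so the drone does not pursue the cursor's position.
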(event EventBeginPlay
  ;[1 1 1] Enable Physics and Collision on the drone
  (Physics|SetSimulatePhysics (Variables|Default|GetPelican) true)
  (Collision|SetCollisionEnabled (Variables|Default|GetPelican) "QueryAndPhysics")
  ;[1 1 1] Calculate Hover Force (To counter gravity)
  (Variables|Default|SetHoverForce (* (Physics|GetMass (Variables|Default|GetPelican)) (Variables|Default|GetGravity))))

(event EventTick
  (params (DeltaSeconds :type Float%20%28single-precision%29))
  (bind _cursor (Variables|Default|GetCursor))
  (bind _pelican (Variables|Default|GetPelican))
  (bind _cursor_2 (Variables|Default|GetCursor))
  (bind _returnvalue (Transformation|GetWorldRotation _cursor_2))
  (bind _returnvalue_2 (Transformation|GetWorldRotation _pelican))
  (bind _returnvalue_3 (Transformation|GetWorldLocation _cursor))
  (bind _returnvalue_4 (Class|KismetMathLibrary|NegateRotator _returnvalue))
  (bind _returnvalue_5 (Math|Rotator|CombineRotators _returnvalue_2 _returnvalue_4))
  (bind _returnvalue_6 (Class|KismetMathLibrary|NegateRotator _returnvalue_5))
  ;[1 1 1] Cursor Debug Arrow
  (Rendering|Debug|DrawDebugArrow _returnvalue_3 (+ _returnvalue_3 (* (Math|Vector|GetForwardVector _cursor) 1e+02)) 1e+01 "(R=1.000000,G=0.010362,B=0.020309,A=1.000000)" 0.0 3.0)
  ;[1 1 1] Cursor Distance Limitation
  (Transformation|SetWorldLocation (Variables|Default|GetCursor) (+ (Math|Vector|ClampVectorSize (- (Transformation|GetWorldLocation (Variables|Default|GetCursor)) (Transformation|GetWorldLocation (Variables|Default|GetPelican))) 0.0 (Variables|Default|GetCursorMaxDistance)) (Transformation|GetWorldLocation (Variables|Default|GetPelican))) false false)
  (Class|PrimitiveComponent|AddTorque (Variables|Default|GetPelican) (Math|Vector|MakeVector 0.0 0.0 (Math|Float|Lerp 0.0 (Variables|Default|GetMaxTorque) (.z (/ (Math|Vector|MakeVector (.roll _returnvalue_6) (.pitch _returnvalue_6) (.yaw _returnvalue_6)) 1.8e+02)))) "None" true)
  (Physics|AddForce (Variables|Default|GetPelican) (Math|Vector|MakeVector 0.0 0.0 (+ 0.0 (Variables|Default|GetHoverForce))) "None" false))

(event Input|AxisEvents|InputAxisMoveForward
  (params (AxisValue :type Float%20%28single-precision%29))
  ;[1 1 1] Cursor Input Control
  (Transformation|AddLocalOffset (Variables|Default|GetCursor) (Math|Vector|MakeVector (* AxisValue 5.0) 0.0 (* (stale Input|AxisEvents|InputAxisMoveUp AxisValue) 5.0)) false false))

(event Input|AxisEvents|InputAxisMoveUp
  (params (AxisValue :type Float%20%28single-precision%29))
  ;[1 1 1] Cursor Input Control
  (Transformation|AddLocalOffset (Variables|Default|GetCursor) (Math|Vector|MakeVector (* (stale Input|AxisEvents|InputAxisMoveForward AxisValue) 5.0) 0.0 (* AxisValue 5.0)) false false))

(event Input|AxisEvents|InputAxisMoveRight
  (params (AxisValue :type Float%20%28single-precision%29))
  ;[1 1 1] Cursor Input Control
  (Transformation|AddLocalRotation (Variables|Default|GetCursor) (Math|Rotator|MakeRotator 0.0 0.0 (* AxisValue 2.0)) false false))

(fn ConstructionScript)